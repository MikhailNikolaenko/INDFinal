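; BP_HandSnap is a VR hand snap point that attaches the player's hand to an object at a set pose.
; SnapHandPosition sends the HandPosition transform, hand skeletal mesh and custom blend space to player character 0 through AttachHandToObjectMessage.
; The construction script shows a preview hand mesh, mirrored on X for left hands.
; At BeginPlay, climbing points enable box collision, and the preview is destroyed unless flagged for runtime display.
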(event EventBeginPlay
  (Utilities|FlowControl|Sequence
    (:then_0
      (if (Variables|Default|GetIsClimbing)
        (Collision|SetCollisionEnabled (Variables|Default|GetBoxCollision) "QueryAndPhysics")))
    (:then_1
      (if (not (Variables|Default|GetDisplay%20preview%20hand%20at%20runtime?))
        (Components|DestroyComponent (Variables|Default|GetStaticMesh))))))

(event EventSnapHandPosition
  (params (Hand%20Skeletal%20Mesh :type B%20Mannequins%20XR%20Object%20Reference))
  (bind _handposition (Variables|Default|GetHandPosition))
  (Class|BPIHandSnapping|AttachHandtoObject(Message) (Game|GetPlayerCharacter 0) (Transformation|GetWorldTransform _handposition) Hand%20Skeletal%20Mesh (Variables|Default|GetCustom%20Anim%20Blend%20Space) _handposition))

(fn ConstructionScript
  (bind _staticmesh (Variables|Default|GetStaticMesh))
  (Components|StaticMesh|SetStaticMesh _staticmesh (Variables|Default|GetHand%20Mesh%20To%20Display))
  (if (Variables|Default|GetIsLeftHand?)
    (Transformation|SetWorldScale3D _staticmesh "-1.000000,1.000000,1.000000")))