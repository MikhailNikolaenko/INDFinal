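; VR joystick actor that a player grabs to send two-axis tilt input to a controlled actor.
; On first-hand grab, it passes the hand mesh to a snap-hand child actor and starts a looping update timer.
; Each update tilts the stick toward the motion controller using look-at dot products, then outputs roll and pitch via JoystickMessage and a dispatcher.
; Release calls a timer pause and recenters the stick.
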(event FirstHandGrabbed(C_GrabComponent)
  (params (Motion%20Controller :type Motion%20Controller%20Component%20Object%20Reference) (SkeltalMeshHand :type B%20Mannequins%20XR%20Object%20Reference))
  (bind _snaphand (Variables|Default|GetSnapHand))
  (bind _childactor (Variables|/Script/Engine.ChildActorComponent|GetChildActor _snaphand))
  (bind _output_get (Variables|Default|SetMotion%20Controller Motion%20Controller))
  (Utilities|Time|SetTimerbyEvent (delegate Custom|Update%20Position) 0.02 true)
  (if (== (Variables|/Script/HeadMountedDisplay.MotionControllerComponent|GetMotionSource _output_get) "Left")
    (Class|BPIHandSnapping|SnapHandPosition(Message) _childactor SkeltalMeshHand)
    (else
      (Class|BPIHandSnapping|SnapHandPosition(Message) _childactor SkeltalMeshHand))))

(event FirstHandDropped(C_GrabComponent)
  (Class|KismetSystemLibrary|PauseTimer 0 "Update Position")
  (Transformation|SetRelativeRotation (Variables|Default|GetJoy%20Stick) "0, 0, 0" false false))

(event Custom|Update%20Position
  (bind _motion_controller (Variables|Default|GetMotion%20Controller))
  (bind _joy_stick (Variables|Default|GetJoy%20Stick))
  (bind _joy_stick_2 (Variables|Default|GetJoy%20Stick))
  (bind _motion_controller_2 (Variables|Default|GetMotion%20Controller))
  (bind _joy_stick_3 (Variables|Default|GetJoy%20Stick))
  (bind _returnvalue (Transformation|GetWorldRotation _joy_stick_2))
  (bind _returnvalue_2 (Transformation|GetWorldLocation _joy_stick_2))
  (bind _returnvalue_3 (Transformation|GetWorldLocation _motion_controller))
  (bind _returnvalue_4 (Transformation|GetWorldRotation _joy_stick))
  (bind _returnvalue_5 (Transformation|GetWorldLocation _joy_stick))
  (bind _returnvalue_6 (Transformation|GetWorldLocation _motion_controller_2))
  (bind _relativerotation (Variables|/Script/Engine.SceneComponent|GetRelativeRotation _joy_stick_3))
  (bind _returnvalue_7 (Math|Rotator|FindLookatRotation _returnvalue_5 _returnvalue_6))
  (bind _returnvalue_8 (Math|Vector|GetForwardVector _returnvalue_4))
  (bind _returnvalue_9 (Math|Vector|GetRightVector _returnvalue))
  (bind _returnvalue_10 (Math|Rotator|FindLookatRotation _returnvalue_2 _returnvalue_3))
  (bind _returnvalue_11 (* (.pitch _relativerotation) -1.0))
  (bind _returnvalue_12 (* (.roll _relativerotation) -1.0))
  (bind _returnvalue_13 (Math|Rotator|GetRotationXVector _returnvalue_7))
  (bind _returnvalue_14 (Math|Rotator|GetRotationXVector _returnvalue_10))
  (bind _returnvalue_15 (* _returnvalue_8 -1.0))
  (bind _returnvalue_16 (Math|Vector|DotProduct _returnvalue_14 _returnvalue_9))
  (bind _returnvalue_17 (Math|Vector|DotProduct _returnvalue_13 _returnvalue_15))
  (bind _returnvalue_18 (* _returnvalue_17 1e+01))
  (bind _returnvalue_19 (* _returnvalue_16 1e+01))
  (bind _returnvalue_20 (Math|Rotator|MakeRotator _returnvalue_19 _returnvalue_18 0.0))
  ;[1 1 1] Calculate left Right Position
  (Transformation|AddRelativeRotation _joy_stick_3 (Math|Rotator|MakeRotator (.roll _returnvalue_20) (.pitch _returnvalue_20) 0.0) false false)
  (Class|BPIPlayerInteractions|Joystick(Message) (Variables|Default|GetActorToControl) _returnvalue_12 _returnvalue_11)
  (Default|CallJoyStickOutputValue _returnvalue_12 _returnvalue_11))

(event EventBeginPlay)

(event Collision|EventActorBeginOverlap
  (params (OtherActor :type Actor%20Object%20Reference)))

(event EventTick
  (params (DeltaSeconds :type Float%20%28single-precision%29)))

(fn ConstructionScript)