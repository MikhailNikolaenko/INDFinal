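; BP_DisplayGazeInteractionExample is an example trigger actor that shows the gaze interaction message while the player is inside its capsule.
; On begin overlap by player character 0, it calls DisplayGazeInteractionMessage on that character's C_GazeInteraction component.
; On end overlap, it hides the message and resets the DoOnce gate that prevents repeated display calls.
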(event OnComponentBeginOverlap(Capsule)
  (params (OverlappedComponent :type Primitive%20Component%20Object%20Reference) (OtherActor :type Actor%20Object%20Reference) (OtherComp :type Primitive%20Component%20Object%20Reference) (OtherBodyIndex :type Integer) (bFromSweep :type Boolean) (SweepResult :type Hit%20Result%20Structure%20%28by%20ref%29))
  (if (== OtherActor (Game|GetPlayerCharacter 0))
    (Utilities|FlowControl|DoOnce false
      (:Completed
        (Class|BPIGazeInteraction|DisplayGazeInteraction(Message) (Actor|GetComponentbyClass (Game|GetPlayerCharacter 0) "/Game/GDXR_VR_Template/Blueprints/Components/GazeInteraction/C_GazeInteraction.C_GazeInteraction_C"))))))

(event OnComponentEndOverlap(Capsule)
  (params (OverlappedComponent :type Primitive%20Component%20Object%20Reference) (OtherActor :type Actor%20Object%20Reference) (OtherComp :type Primitive%20Component%20Object%20Reference) (OtherBodyIndex :type Integer))
  (bind _returnvalue (Game|GetPlayerCharacter 0))
  (bind _returnvalue_2 (Actor|GetComponentbyClass _returnvalue "/Game/GDXR_VR_Template/Blueprints/Components/GazeInteraction/C_GazeInteraction.C_GazeInteraction_C"))
  (if (== OtherActor (Game|GetPlayerCharacter 0))
    (Class|BPIGazeInteraction|HideGazeInteraction(Message) _returnvalue_2)
    (Utilities|FlowControl|DoOnce false) ; enters at Reset
  ))

(fn ConstructionScript)