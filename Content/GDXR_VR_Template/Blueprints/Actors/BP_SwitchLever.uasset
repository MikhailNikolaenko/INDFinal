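; BP_SwitchLever is a grabbable VR lever that drives a linked ActorToActivate and broadcasts its state.
; Grabbing snaps the hand on and starts a looping timer that pitches the switch toward the motion controller within clamped limits, broadcasting the gradient.
; On release, optional SnapOnOff snaps to either limit, sends ActivateMessage and broadcasts on/off.
; The construction script also messages the target from the initial pitch, with opposite polarity to release.
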(event FirstHandGrabbed(C_GrabComponent)
  (params (Motion%20Controller :type Motion%20Controller%20Component%20Object%20Reference) (SkeltalMeshHand :type B%20Mannequins%20XR%20Object%20Reference))
  (Variables|Default|SetMotion%20Controller Motion%20Controller)
  (Utilities|Time|SetTimerbyEvent (delegate Custom|Update%20Rotation) 0.02 true)
  ;[1 1 1] Snap Hand
  (Class|BPIHandSnapping|SnapHandPosition(Message) (Variables|/Script/Engine.ChildActorComponent|GetChildActor (Variables|Default|GetSnapHand)) SkeltalMeshHand))

(event FirstHandDropped(C_GrabComponent)
  (bind _switch (Variables|Default|GetSwitch))
  (bind _actor_to_activate (Variables|Default|GetActor%20To%20Activate))
  (Class|KismetSystemLibrary|PauseTimer 0 "Update Rotation")
  (Variables|Default|SetMotion%20Controller 0)
  (if (Variables|Default|GetSnap%20On%20Off)
    (if (> (.pitch (Variables|/Script/Engine.SceneComponent|GetRelativeRotation (Variables|Default|GetSwitch))) 0.0)
      (Transformation|SetRelativeRotation _switch (Math|Rotator|MakeRotator 0.0 3e+01 0.0) true false)
      (Class|BPIPlayerInteractions|Activate(Message) _actor_to_activate true)
      (Default|CallSwitchLeverSnaponOff true)
      (else
        (Transformation|SetRelativeRotation _switch (Math|Rotator|MakeRotator 0.0 -3e+01 0.0) true false)
        (Class|BPIPlayerInteractions|Activate(Message) _actor_to_activate false)
        (Default|CallSwitchLeverSnaponOff false)))))

(event Custom|Update%20Rotation
  (bind _switch (Variables|Default|GetSwitch))
  (Transformation|SetRelativeRotation _switch (Math|Rotator|MakeRotator 0.0 (Math|Float|ClampAngle (.pitch (Math|Rotator|FindLookatRotation (Transformation|GetWorldLocation (Variables|Default|GetSwitch)) (Transformation|GetWorldLocation (stale FirstHandGrabbed(C_GrabComponent) Motion%20Controller)))) -3e+01 3e+01) 0.0) true false)
  (Default|CallSwitchLeverGradient (.pitch (Variables|/Script/Engine.SceneComponent|GetRelativeRotation _switch))))

(fn ConstructionScript
  (bind _actor_to_activate (Variables|Default|GetActor%20To%20Activate))
  (if (> (.pitch (Variables|/Script/Engine.SceneComponent|GetRelativeRotation (Variables|Default|GetSwitch))) 0.0)
    (Class|BPIPlayerInteractions|Activate(Message) _actor_to_activate false)
    (else
      (Class|BPIPlayerInteractions|Activate(Message) _actor_to_activate true))))