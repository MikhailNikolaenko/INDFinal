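; BP_BodyItemStorage is a VR body holster with left and right item storage slots that can follow the player.
; With auto-attach on, it snaps to the player, and a looping timer places it below the camera by the capsule half-height, interpolating only yaw toward the camera's.
; On BeginPlay it also spawns a pistol and a two-hand rifle as default items for the child BP_SingleItemStorage actors.
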(event Custom|Update%20Holster%20Rotation
  (bind _returnvalue (Game|GetPlayerCharacter 0))
  (bind _defaultsceneroot (Variables|Default|GetDefaultSceneRoot))
  (bind _returnvalue_2 (Actor|GetComponentbyClass _returnvalue "/Script/Engine.CameraComponent"))
  (bind _returnvalue_3 (Transformation|GetWorldLocation _returnvalue_2))
  (Transformation|SetWorldRotation _defaultsceneroot (Math|Rotator|MakeRotator 0.0 0.0 (.yaw (Math|Interpolation|RInterpTo (Transformation|GetWorldRotation _defaultsceneroot) (Transformation|GetWorldRotation _returnvalue_2) (Class|KismetSystemLibrary|GetTimerElapsedTimeHandle (stale EventBeginPlay _returnvalue)) 1.0))) false false)
  (Transformation|SetWorldLocation _defaultsceneroot (Math|Vector|MakeVector (.x _returnvalue_3) (.y _returnvalue_3) (- (.z _returnvalue_3) (Variables|/Script/Engine.CapsuleComponent|GetCapsuleHalfHeight (Actor|GetComponentbyClass _returnvalue "/Script/Engine.CapsuleComponent")))) true false))

(event EventBeginPlay
  (if (Variables|Default|GetAutoAttachToPlayer?)
    (Transformation|AttachActorToActor (Game|GetPlayerCharacter 0) "None" "SnapToTarget" "SnapToTarget" "SnapToTarget" true)
    (bind _returnvalue (Utilities|Time|SetTimerbyEvent (delegate Custom|Update%20Holster%20Rotation) 0.02 true)))
  ;[1 1 1] Spawn Default Actors
  (Utilities|FlowControl|Sequence
    (:then_0
      (bind _returnvalue_2 (Game|SpawnActorfromClass "/Game/GDXR_VR_Template/Blueprints/Actors/BP_Pistol.BP_Pistol_C" (Math|Transform|MakeTransform "0, 0, 0" "0, 0, 0" "1.000000,1.000000,1.000000") "AlwaysSpawn" 0 0))
      (Default|CallSetDefaultItem (.AsBP%20Single%20Item%20Storage (Utilities|Casting|CastToBP_SingleItemStorage (Variables|/Script/Engine.ChildActorComponent|GetChildActor (Variables|Default|GetLeftStorage)))) _returnvalue_2))
    (:then_1
      (bind _returnvalue_3 (Game|SpawnActorfromClass "/Game/GDXR_VR_Template/Blueprints/Actors/BP_TwoHandRifle.BP_TwoHandRifle_C" (Math|Transform|MakeTransform "0, 0, 0" "0, 0, 0" "1.000000,1.000000,1.000000") "AlwaysSpawn" 0 0))
      (Default|CallSetDefaultItem (.AsBP%20Single%20Item%20Storage (Utilities|Casting|CastToBP_SingleItemStorage (Variables|/Script/Engine.ChildActorComponent|GetChildActor (Variables|Default|GetRightStorage)))) _returnvalue_3))))

(fn ConstructionScript)